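; BP_Dish is a dish actor for a food assembly mechanic with sushi ingredients, currently running as a timed test sequence.
; On BeginPlay it calls functions to add rice, seaweed, cucumber and salmon in that order, each after a short delay.
; It prints the Key variable after each addition; the add functions are not defined in these graphs, and overlap, tick and construction logic are empty.
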(event EventBeginPlay
  (bind _key (Variables|Default|GetKey))
  (Utilities|FlowControl|Delay 2.0)
  (Class|DishActor|AddRice)
  (Development|PrintString _key)
  (Utilities|FlowControl|Delay 2.0)
  (Class|DishActor|AddSeaWeed)
  (Development|PrintString _key)
  (Utilities|FlowControl|Delay 2.0)
  (Class|DishActor|AddCucumber)
  (Development|PrintString _key)
  (Utilities|FlowControl|Delay 2.0)
  (Class|DishActor|AddSalmon)
  (Development|PrintString _key))

(event Collision|EventActorBeginOverlap
  (params (OtherActor :type Actor%20Object%20Reference)))

(event EventTick
  (params (DeltaSeconds :type Float%20%28single-precision%29)))

(fn ConstructionScript)